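; BP_staircase is an interactable staircase actor that loads level01 when F is pressed.
; On BeginPlay it creates a hidden HUD_F widget, which its Box collision shows on overlap and hides when the overlap ends.
; Both overlap events call EnableInput for player 0 without filtering the overlapping actor, so F stays active after the player leaves the box.
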(event OnComponentBeginOverlap(Box)
  (params (OverlappedComponent :type Primitive%20Component%20Object%20Reference) (OtherActor :type Actor%20Object%20Reference) (OtherComp :type Primitive%20Component%20Object%20Reference) (OtherBodyIndex :type Integer) (bFromSweep :type Boolean) (SweepResult :type Hit%20Result%20Structure%20%28by%20ref%29))
  (Input|EnableInput (Game|GetPlayerController 0))
  (Widget|SetVisibility (Variables|Default|GetHUD_F) "Visible"))

(event OnComponentEndOverlap(Box)
  (params (OverlappedComponent :type Primitive%20Component%20Object%20Reference) (OtherActor :type Actor%20Object%20Reference) (OtherComp :type Primitive%20Component%20Object%20Reference) (OtherBodyIndex :type Integer))
  (Input|EnableInput (Game|GetPlayerController 0))
  (Widget|SetVisibility (Variables|Default|GetHUD_F) "Hidden"))

(event EventBeginPlay
  (bind _returnvalue (UserInterface|CreateWidget "/Game/Project/BP/HUD_F.HUD_F_C"))
  (bind _output_get (Variables|Default|SetHUD_F _returnvalue))
  (UserInterface|Viewport|AddtoViewport _output_get 0)
  (Widget|SetVisibility _output_get "Hidden"))

(event Collision|EventActorBeginOverlap
  (params (OtherActor :type Actor%20Object%20Reference)))

(event EventTick
  (params (DeltaSeconds :type Float%20%28single-precision%29)))

(event Input|KeyboardEvents|F
  (params (Key :type Key%20Structure :default "None"))
  (:Pressed
    (Game|OpenLevel(byName) "level01")))

(fn ConstructionScript)
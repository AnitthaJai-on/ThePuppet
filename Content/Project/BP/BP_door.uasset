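; BP_door is an interactive door that F toggles by playing or reversing a timeline driving its world yaw.
; A box overlap shows or hides the HUD_F widget; both begin and end enable input, so it is never disabled.
; A BP_close_door actor spawns at a hard-coded transform on BeginPlay, then is respawned or destroyed with each toggle.
; The timeline update also hides the prompt.
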(event OnComponentBeginOverlap(Box)
  (params (OverlappedComponent :type Primitive%20Component%20Object%20Reference) (OtherActor :type Actor%20Object%20Reference) (OtherComp :type Primitive%20Component%20Object%20Reference) (OtherBodyIndex :type Integer) (bFromSweep :type Boolean) (SweepResult :type Hit%20Result%20Structure%20%28by%20ref%29))
  ;[1 1 1] In/Out box
  (Input|EnableInput (Game|GetPlayerController 0))
  ;[1 1 1] Show/Hidden HID F
  (Widget|SetVisibility (Variables|Default|GetHUD_F) "Visible"))

(event OnComponentEndOverlap(Box)
  (params (OverlappedComponent :type Primitive%20Component%20Object%20Reference) (OtherActor :type Actor%20Object%20Reference) (OtherComp :type Primitive%20Component%20Object%20Reference) (OtherBodyIndex :type Integer))
  ;[1 1 1] In/Out box
  (Input|EnableInput (Game|GetPlayerController 0))
  ;[1 1 1] Show/Hidden HID F
  (Widget|SetVisibility (Variables|Default|GetHUD_F) "Hidden"))

(event EventBeginPlay
  ;[1 1 1] open game spaw close door
  (bind _returnvalue (Game|SpawnActorfromClass "/Game/Project/BP/BP_close_door.BP_close_door_C" (Math|Transform|MakeTransform "180.000000,130.000000,100.000000" "0.000000,0.000000,-90.000000" "-1.500000,2.750000,1.000000") "Undefined" 0 0))
  (Variables|Default|SetClose_door _returnvalue)
  (bind _returnvalue_2 (UserInterface|CreateWidget "/Game/Project/BP/HUD_F.HUD_F_C"))
  (bind _output_get (Variables|Default|SetHUD_F _returnvalue_2))
  (UserInterface|Viewport|AddtoViewport _output_get 0)
  (Widget|SetVisibility _output_get "Hidden"))

(event Input|KeyboardEvents|F
  (params (Key :type Key%20Structure :default "None"))
  ;[1 1 1] Open/Close
  (:Pressed
    (if (Variables|Default|Getclose)
      (Variables|Default|Setclose false)
      (bind _returnvalue (Game|SpawnActorfromClass "/Game/Project/BP/BP_close_door.BP_close_door_C" (Math|Transform|MakeTransform "180.000000,130.000000,100.000000" "0, 0,-90.000000" "-1.500000,2.750000,1") "Undefined" 0 0))
      (Variables|Default|SetClose_door _returnvalue)
      (bind _o_c (Timeline|O/C Play)
        (:Update
          (Transformation|SetWorldRotation (Variables|Default|Getdoor) (Math|Rotator|MakeRotator 0.0 0.0 _o_c) false false)
          (Widget|SetVisibility (Variables|Default|GetHUD_F) "Hidden")))
      (else
        (Variables|Default|Setclose true)
        (Actor|DestroyActor (Variables|Default|GetClose_door))
        (Timeline|O/C Reverse)))))

(fn ConstructionScript)
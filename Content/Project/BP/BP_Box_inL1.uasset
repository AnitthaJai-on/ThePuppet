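; Trigger box, apparently for an interior area of L1, that swaps which of two wall-face actors is visible when something overlaps it.
; BeginPlay spawns both walls at hard-coded transforms, stores them as WellIn and WellOut, and hides the WellOut root component.
; Overlap begin hides the WellIn mesh and shows WellOut, and overlap end reverses this.
; Both overlap events also enable input for player 0, with no check on the overlapping actor.
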(event OnComponentBeginOverlap(CollisionComponent)
  (params (OverlappedComponent :type Primitive%20Component%20Object%20Reference) (OtherActor :type Actor%20Object%20Reference) (OtherComp :type Primitive%20Component%20Object%20Reference) (OtherBodyIndex :type Integer) (bFromSweep :type Boolean) (SweepResult :type Hit%20Result%20Structure%20%28by%20ref%29))
  (Input|EnableInput (Game|GetPlayerController 0))
  (Rendering|SetVisibility (Variables|/Script/Engine.StaticMeshActor|GetStaticMeshComponent (Variables|Default|GetWell_in)) false false)
  (Rendering|SetVisibility (Variables|/Script/Engine.StaticMeshActor|GetStaticMeshComponent (Variables|Default|GetWell_out)) true false))

(event OnComponentEndOverlap(CollisionComponent)
  (params (OverlappedComponent :type Primitive%20Component%20Object%20Reference) (OtherActor :type Actor%20Object%20Reference) (OtherComp :type Primitive%20Component%20Object%20Reference) (OtherBodyIndex :type Integer))
  (Input|EnableInput (Game|GetPlayerController 0))
  (Rendering|SetVisibility (Variables|/Script/Engine.StaticMeshActor|GetStaticMeshComponent (Variables|Default|GetWell_in)) true false)
  (Rendering|SetVisibility (Variables|/Script/Engine.StaticMeshActor|GetStaticMeshComponent (Variables|Default|GetWell_out)) false false))

(event EventBeginPlay
  (bind _returnvalue (Game|SpawnActorfromClass "/Game/Project/BP/BP_Wall_Face_inL1.BP_Wall_Face_inL1_C" (Math|Transform|MakeTransform "750.000000,150.000000,10.000000" "0,-90.000000,0.000000" "3.250000,1.000000,2.250000") "Undefined" 0 0))
  (Variables|Default|SetWell_in _returnvalue)
  (bind _returnvalue_2 (Game|SpawnActorfromClass "/Game/Project/BP/BP_Wall_Face_L1.BP_Wall_Face_L1_C" (Math|Transform|MakeTransform "390.000000,1110.000000,10.000000" "0,-90.000000,0.000000" "1,1,1") "Undefined" 0 0))
  (bind _output_get (Variables|Default|SetWell_out _returnvalue_2))
  (Rendering|SetVisibility (Variables|/Script/Engine.Actor|GetRootComponent _output_get) false false))

(fn ConstructionScript)
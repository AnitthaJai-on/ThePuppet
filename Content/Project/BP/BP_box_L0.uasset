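; BP_box_L0 is a trigger box that swaps the visibility of two walls it spawns at fixed transforms on BeginPlay.
; Wall0 starts hidden; any overlap with CollisionComponent shows it and hides Wall1, and ending the overlap reverses this.
; Only root component visibility changes, without propagating to children or altering collision.
; Overlap also enables input from player controller 0, though the event graph has no input events.
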(event OnComponentBeginOverlap(CollisionComponent)
  (params (OverlappedComponent :type Primitive%20Component%20Object%20Reference) (OtherActor :type Actor%20Object%20Reference) (OtherComp :type Primitive%20Component%20Object%20Reference) (OtherBodyIndex :type Integer) (bFromSweep :type Boolean) (SweepResult :type Hit%20Result%20Structure%20%28by%20ref%29))
  (Input|EnableInput (Game|GetPlayerController 0))
  (Rendering|SetVisibility (Variables|/Script/Engine.Actor|GetRootComponent (Variables|Default|Getwall0)) true false)
  (Rendering|SetVisibility (Variables|/Script/Engine.Actor|GetRootComponent (Variables|Default|Getwall1)) false false))

(event OnComponentEndOverlap(CollisionComponent)
  (params (OverlappedComponent :type Primitive%20Component%20Object%20Reference) (OtherActor :type Actor%20Object%20Reference) (OtherComp :type Primitive%20Component%20Object%20Reference) (OtherBodyIndex :type Integer))
  (Rendering|SetVisibility (Variables|/Script/Engine.Actor|GetRootComponent (Variables|Default|Getwall0)) false false)
  (Rendering|SetVisibility (Variables|/Script/Engine.Actor|GetRootComponent (Variables|Default|Getwall1)) true false))

(event EventBeginPlay
  (bind _returnvalue (Game|SpawnActorfromClass "/Game/Project/BP/BP_Wall.BP_Wall_C" (Math|Transform|MakeTransform "300.000000,140.000000,-15.000000" "0,90.000000, 0" "2.000000,1,1.750000") "Undefined" 0 0))
  (bind _output_get (Variables|Default|Setwall0 _returnvalue))
  (bind _returnvalue_2 (Game|SpawnActorfromClass "/Game/Project/BP/BP_Wall.BP_Wall_C" (Math|Transform|MakeTransform "870.000000,-130.000000,-50.000000" "0,90.000000, 0" "0.750000,1,1.750000") "Undefined" 0 0))
  (Variables|Default|Setwall1 _returnvalue_2)
  (Rendering|SetVisibility (Variables|/Script/Engine.Actor|GetRootComponent _output_get) false false))

(fn ConstructionScript)
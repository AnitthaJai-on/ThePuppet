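; An overlap-triggered Blueprint that shows the HUD_Q widget while something is inside its CollisionComponent.
; BeginPlay creates the widget hidden, and begin and end overlap toggle its visibility without checking which actor overlapped.
; Both overlap events call EnableInput for player controller 0, so input stays enabled after leaving.
; The F key sets a Value boolean while held, which nothing in these graphs reads.
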(event OnComponentBeginOverlap(CollisionComponent)
  (params (OverlappedComponent :type Primitive%20Component%20Object%20Reference) (OtherActor :type Actor%20Object%20Reference) (OtherComp :type Primitive%20Component%20Object%20Reference) (OtherBodyIndex :type Integer) (bFromSweep :type Boolean) (SweepResult :type Hit%20Result%20Structure%20%28by%20ref%29))
  (Input|EnableInput (Game|GetPlayerController 0))
  (Widget|SetVisibility (Variables|Default|GetHUD_Q) "Visible"))

(event OnComponentEndOverlap(CollisionComponent)
  (params (OverlappedComponent :type Primitive%20Component%20Object%20Reference) (OtherActor :type Actor%20Object%20Reference) (OtherComp :type Primitive%20Component%20Object%20Reference) (OtherBodyIndex :type Integer))
  (Input|EnableInput (Game|GetPlayerController 0))
  (Widget|SetVisibility (Variables|Default|GetHUD_Q) "Hidden"))

(event EventBeginPlay
  (bind _returnvalue (UserInterface|CreateWidget "/Game/Project/BP/HUD_Q.HUD_Q_C"))
  (bind _output_get (Variables|Default|SetHUD_Q _returnvalue))
  (UserInterface|Viewport|AddtoViewport _output_get 0)
  (Widget|SetVisibility _output_get "Hidden"))

(event Input|KeyboardEvents|F
  (params (Key :type Key%20Structure :default "None"))
  (:Pressed
    (Variables|Default|Setvalue true))
  (:Released
    (Variables|Default|Setvalue false)))

(fn ConstructionScript)